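; Menu cube that opens TutorialMap when a trace dwells on it for two seconds or activates it with a press.
; Trace callbacks flag hits on the cube and move an arrow to the hit point and normal.
; Tick accumulates dwell time into a dynamic ring material's fill, tints the cube, and resets both when the hit ends.
; The ring billboards toward the player pawn each frame.
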(event EventBeginPlay)

(event Collision|EventActorBeginOverlap
  (params (OtherActor :type Actor%20Object%20Reference)))

(event EventTick
  (params (DeltaSeconds :type Float%20%28single-precision%29))
  (bind _cube (Variables|Default|GetCube))
  (CallFunction|BillboardFunction)
  ;[1 1 1] Check if hits
  (if (Variables|Default|GetinHit)
    (Rendering|Material|SetVectorParameterValueonMaterials (Variables|Default|GetCube) "Color" "0.200000,0.150000,0.500000")
    ;[1 1 1] If hit, sum the seconds to the counter
    (bind _output_get (Variables|Default|SetsecondsCont (+ DeltaSeconds (Variables|Default|GetsecondsCont))))
    ;[1 1 1] Create Dynamic material
    (bind _returnvalue (Rendering|Material|CreateDynamicMaterialInstance (Variables|Default|GetFuseBtn) 0 "/Game/Tutorial/UIRing_2.UIRing_2" :!class /Script/Engine.PrimitiveComponent))
    (bind _output_get_2 (Variables|Default|SetRingDynamic _returnvalue))
    (Rendering|Material|SetMaterial (Variables|Default|GetFuseBtn) 0 _output_get_2)
    ;[1 1 1] Fill the porcentage of the dynamic ring
    (if (>= _output_get 2.0)
      (Game|OpenLevel(byName) "TutorialMap")
      (else
        (Rendering|Material|SetScalarParameterValueonMaterials (Variables|Default|GetFuseBtn) "PercentComplete" (/ _output_get 2.0))))
    (else
      ;[1 1 1] If not hitting restart the counter and color
      (CallFunction|RestartCounter)
      (if (Variables|Default|GetisActivated)
        (Rendering|Material|SetVectorParameterValueonMaterials _cube "Color" "1.000000,1.000000,0.000000")
        (else
          (Rendering|Material|SetVectorParameterValueonMaterials _cube "Color" "1.000000,1.000000,1.000000"))))))

(fn ConstructionScript)

(fn BillboardFunction
  (Transformation|SetWorldRotation (Variables|Default|GetFuseBtn) (Math|Rotator|FindLookatRotation (Transformation|GetWorldLocation (Variables|Default|GetFuseBtn)) (Transformation|GetActorLocation (Game|Player|GetPlayerPawn 0))) false false))

(fn ChangeColor
  (bind _cube (Variables|Default|GetCube))
  ;[1 1 1] Change the color of the cube
  (if (Variables|Default|GetisActivated)
    (Rendering|Material|SetVectorParameterValueonMaterials _cube "Color" "1.000000,1.000000,1.000000")
    (Variables|Default|SetisActivated false)
    (else
      (Rendering|Material|SetVectorParameterValueonMaterials _cube "Color" "1.000000,1.000000,0.000000")
      (Variables|Default|SetisActivated true)))
  ;[1 1 1] Restart counter and stop hitting
  (CallFunction|RestartCounter))

(fn RestartCounter
  (bind _output_get (Variables|Default|SetsecondsCont 0.0))
  (Rendering|Material|SetScalarParameterValueonMaterials (Variables|Default|GetFuseBtn) "PercentComplete" _output_get)
  (Variables|Default|SetinHit false))

(fn TraceActivateDown
  (params (Hit :type Hit%20Result%20Structure) (Instigator :type Pawn%20Object%20Reference))
  (Game|OpenLevel(byName) "TutorialMap")
  (return false))

(fn TraceActivateUp
  (params (Hit :type Hit%20Result%20Structure) (Instigator :type Pawn%20Object%20Reference))
  (return false))

(fn TraceHitComponent
  (params (Hit :type Hit%20Result%20Structure) (Component :type Primitive%20Component%20Object%20Reference))
  ;[1 1 1] Take into account the hit if it is in the cube
  (if (== Component (Variables|Default|GetCube))
    (Variables|Default|SetinHit true))
  (return false))

(fn TraceHitObject
  (params (Hit :type Hit%20Result%20Structure))
  (return false))

(fn TraceLeaveComponent
  (params (Hit :type Hit%20Result%20Structure) (Component :type Primitive%20Component%20Object%20Reference))
  ;[1 1 1] Take into account the hit if it is leaving the cube
  (if (== Component (Variables|Default|GetCube))
    (Variables|Default|SetinHit false))
  (return false))

(fn TraceLeaveObject
  (params (Hit :type Hit%20Result%20Structure))
  (Variables|Default|SetinHit false)
  (return false))

(fn TraceMove
  (params (Hit :type Hit%20Result%20Structure%20%28by%20ref%29))
  (bind (_bblockinghit _binitialoverlap _time _distance _location _impactpoint _normal _impactnormal _physmat _hitactor _hitcomponent) (Collision|BreakHitResult Hit))
  ;[1 1 1] Only move the arrow into the cube
  (if (== (Variables|Default|GetCube) _hitcomponent)
    (Transformation|SetWorldLocationAndRotation (Variables|Default|GetArrow) _location (Math|Rotator|MakeRotfromX _normal) false false)
    (return false)))